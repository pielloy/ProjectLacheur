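; BP_EditorButtons is a map editor actor that provides a pair of add and remove tile buttons for one direction of the map.
; On BeginPlay it spawns and attaches two BP_EditorButton actors on either side of itself, each with its own material, IsAdd flag and back-reference to this actor.
; Its OnClick function forwards the add/remove choice, together with its Dir, to the Map's OnClick.
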(event EventBeginPlay
  (bind _returnvalue (Game|SpawnActorfromClass "/Game/MapEditorAssets/EditorMap/Blueprints/Tile/BP_EditorButton.BP_EditorButton_C" (Math|Transform|MakeTransform "-50.000000, 0, 0" "0, 0, 0" "0.600000,0.600000,1") "Undefined" 0 0))
  (Transformation|AttachActorToActor _returnvalue self "None" "KeepRelative" "SnapToTarget" "KeepRelative" true)
  (Rendering|Material|SetMaterial (Variables|/Game/MapEditorAssets/EditorMap/Blueprints/Tile/BP_EditorButton.BP_EditorButton_C|GetPlane _returnvalue) 0 "/Game/MapEditorAssets/EditorMap/Materials/MI_RemoveTile.MI_RemoveTile")
  (Variables|/Game/MapEditorAssets/EditorMap/Blueprints/Tile/BP_EditorButton.BP_EditorButton_C|SetIsAdd? _returnvalue false)
  (Variables|/Game/MapEditorAssets/EditorMap/Blueprints/Tile/BP_EditorButton.BP_EditorButton_C|SetEditorButtons _returnvalue self)
  (bind _returnvalue_2 (Game|SpawnActorfromClass "/Game/MapEditorAssets/EditorMap/Blueprints/Tile/BP_EditorButton.BP_EditorButton_C" (Math|Transform|MakeTransform "50.000000, 0, 0" "0, 0, 0" "0.600000,0.600000,1") "Undefined" 0 0))
  (Transformation|AttachActorToActor _returnvalue_2 self "None" "KeepRelative" "SnapToTarget" "KeepRelative" true)
  (Rendering|Material|SetMaterial (Variables|/Game/MapEditorAssets/EditorMap/Blueprints/Tile/BP_EditorButton.BP_EditorButton_C|GetPlane _returnvalue_2) 0 "/Game/MapEditorAssets/EditorMap/Materials/MI_AddTile.MI_AddTile")
  (Variables|/Game/MapEditorAssets/EditorMap/Blueprints/Tile/BP_EditorButton.BP_EditorButton_C|SetIsAdd? _returnvalue_2 true)
  (Variables|/Game/MapEditorAssets/EditorMap/Blueprints/Tile/BP_EditorButton.BP_EditorButton_C|SetEditorButtons _returnvalue_2 self))

(fn ConstructionScript)

(fn OnClick
  (params (Add :type Boolean))
  (Default|OnClick (Variables|Default|GetMap) (Variables|Default|GetDir) Add))