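; BP_EditorMap is a map editor actor that builds a small centered grid of BP_EditorTile actors with resize-style buttons around it.
; On BeginPlay it spawns and attaches the tiles, then creates four directional BP_EditorButtons referencing itself and positions them beyond the grid edges.
; Button clicks route through OnClick, but only PlusX is handled and its body is empty.
; Construction creates a MultiDimentionalMap object that the graphs never fill.
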(event EventBeginPlay
  (Init|GenerateMap)
  (Init|InitButons)
  (CallFunction|MoveButtons))

(event Collision|EventActorBeginOverlap
  (params (OtherActor :type Actor%20Object%20Reference)))

(event EventTick
  (params (DeltaSeconds :type Float%20%28single-precision%29)))

(fn ConstructionScript
  (bind _returnvalue (Game|ConstructObjectfromClass "/Script/ProjectLacheur.MultiDimentionalMap" self))
  (Variables|Default|SetMap _returnvalue))

(fn GenerateMap
  (Variables|Default|SetWidth 2)
  (Variables|Default|SetHeight 2)
  (for _index (range 0 2)
    (for _index_2 (range 0 2)
      (Init|SpawnTileGeneration _index_2 _index))))

(fn SpawnTileGeneration
  (params (Pos%20X :type Integer) (Pos%20Y :type Integer))
  (bind _returnvalue (Game|SpawnActorfromClass "/Game/MapEditorAssets/EditorMap/Blueprints/Tile/BP_EditorTile.BP_EditorTile_C" (Math|Transform|MakeTransform (Math|Vector|MakeVector (- (* (Math|Conversions|ToFloat(Integer) Pos%20X) 1e+02) (* (/ (Math|Conversions|ToFloat(Integer) (Variables|Default|GetWidth)) 2.0) 1e+02)) (- (* (Math|Conversions|ToFloat(Integer) Pos%20Y) 1e+02) (* (/ (Math|Conversions|ToFloat(Integer) (Variables|Default|GetHeight)) 2.0) 1e+02)) 0.0) "0, 0, 0" "0.800000,0.800000,0.100000") "Undefined" 0 0))
  (Transformation|AttachActorToActor _returnvalue self "None" "KeepRelative" "KeepRelative" "KeepRelative" true)
  (return _returnvalue))

(fn MoveButtons
  (Transformation|SetRelativeLocation (Variables|/Script/Engine.Actor|GetRootComponent (Variables|Buttons|GetButtonMinusY)) (Math|Vector|MakeVector 0.0 (+ (* (/ (Math|Conversions|ToFloat(Integer) (Variables|Default|GetHeight)) 2.0) 1e+02) 1.5e+02) 0.0) false false)
  (Transformation|SetRelativeLocation (Variables|/Script/Engine.Actor|GetRootComponent (Variables|Buttons|GetButtonsMinusX)) (Math|Vector|MakeVector (+ (* (/ (Math|Conversions|ToFloat(Integer) (Variables|Default|GetWidth)) 2.0) 1e+02) 1.5e+02) 0.0 0.0) false false)
  (Transformation|SetRelativeLocation (Variables|/Script/Engine.Actor|GetRootComponent (Variables|Buttons|GetButtonPlusY)) (Math|Vector|MakeVector 0.0 (+ (* (/ (Math|Conversions|ToFloat(Integer) (Variables|Default|GetHeight)) 2.0) -1e+02) -1.5e+02) 0.0) false false)
  (Transformation|SetRelativeLocation (Variables|/Script/Engine.Actor|GetRootComponent (Variables|Buttons|GetButtonsPlusX)) (Math|Vector|MakeVector (+ (* (/ (Math|Conversions|ToFloat(Integer) (Variables|Default|GetWidth)) 2.0) -1e+02) -1.5e+02) 0.0 0.0) false false))

(fn InitButons
  (bind _ret (CallFunction|CreateButton 9e+01 "NewEnumerator0"))
  (Variables|Buttons|SetButtonsPlusX _ret)
  (bind _ret_2 (CallFunction|CreateButton -9e+01 "NewEnumerator1"))
  (Variables|Buttons|SetButtonsMinusX _ret_2)
  (bind _ret_3 (CallFunction|CreateButton 1.8e+02 "NewEnumerator2"))
  (Variables|Buttons|SetButtonPlusY _ret_3)
  (bind _ret_4 (CallFunction|CreateButton 0.0 "NewEnumerator3"))
  (Variables|Buttons|SetButtonMinusY _ret_4))

(fn CreateButton
  (params (Rotation :type Float%20%28single-precision%29) (Dir :type E_EditorEnumDir%20Enum :default "NewEnumerator0"))
  (bind _returnvalue (Game|SpawnActorfromClass "/Game/MapEditorAssets/EditorMap/Blueprints/BP_EditorButtons.BP_EditorButtons_C" (Math|Transform|MakeTransform "0, 0, 0" (Math|Rotator|MakeRotator 0.0 0.0 Rotation) "1,1,1") "Undefined" 0 0))
  (Variables|/Game/MapEditorAssets/EditorMap/Blueprints/BP_EditorButtons.BP_EditorButtons_C|SetDir _returnvalue Dir)
  (Variables|/Game/MapEditorAssets/EditorMap/Blueprints/BP_EditorButtons.BP_EditorButtons_C|SetMap _returnvalue self)
  (return _returnvalue))

(fn OnClick
  (params (Dir :type E_EditorEnumDir%20Enum :default "NewEnumerator0") (Plus :type Boolean))
  (switch Utilities|FlowControl|Switch|SwitchonE_EditorEnumDir Dir
    (:NewEnumerator0
      (ResizeMap|PlusX Plus))))

(fn PlusX
  (params (Add :type Boolean))
  (if Add
    _))

(fn SpawnTile
  (params (Location :type Vector))
  (bind _returnvalue (Game|SpawnActorfromClass "/Game/MapEditorAssets/EditorMap/Blueprints/Tile/BP_EditorTile.BP_EditorTile_C" (Math|Transform|MakeTransform Location "0, 0, 0" "0.800000,0.800000,0.100000") "Undefined" 0 0))
  (Transformation|AttachActorToActor _returnvalue self "None" "KeepRelative" "KeepRelative" "KeepRelative" true)
  (return _returnvalue))