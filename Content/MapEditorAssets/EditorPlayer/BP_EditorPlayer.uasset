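; Player for the map editor that shows the mouse cursor, creates the editor UI and drives camera and tile selection.
; Each tick a cursor trace looks for actors implementing BPI_EditorTileInteraction, tracking the hovered tile and switching its focus.
; The Click input forwards OnClick to that tile.
; Axis inputs pan the SpringArm along world diagonals while right mouse is held, and the wheel zooms by changing arm length.
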(event EventBeginPlay
  (Utilities|FlowControl|Sequence
    (:then_0
      (|Showcursor))
    (:then_1
      (UserInterface|CreateWidget))))

(event EventTick
  (params (DeltaSeconds :type Float%20%28single-precision%29))
  (|SelectedCase))

(fn ConstructionScript)

(event Input|ActionEvents|InputActionClick
  (params (Key :type Key%20Structure))
  (bind _mouseselectedtile (Variables|Default|GetMouseSelectedTile))
  (:Pressed
    (if (!= 0 (Utilities|ToObject(Interface) _mouseselectedtile))
      (Default|OnClick _mouseselectedtile))))

(event Input|AxisEvents|InputAxisUp
  (params (AxisValue :type Float%20%28single-precision%29))
  (bind _springarm (Variables|Default|GetSpringArm))
  ;[1 1 1] Movement
  (if (Variables|Default|GetCanMove?)
    (Transformation|SetWorldLocation _springarm (+ (Transformation|GetWorldLocation _springarm) (* "1.000000,1.000000, 0" (* AxisValue (Variables|Default|GetCameraSpeed)))) false false)))

(event Input|AxisEvents|InputAxisRight
  (params (AxisValue :type Float%20%28single-precision%29))
  (bind _springarm (Variables|Default|GetSpringArm))
  ;[1 1 1] Movement
  (if (Variables|Default|GetCanMove?)
    (Transformation|SetWorldLocation _springarm (+ (Transformation|GetWorldLocation _springarm) (* "1.000000,-1.000000, 0" (* AxisValue (Variables|Default|GetCameraSpeed)))) false false)))

(event Input|MouseEvents|RightMouseButton
  (params (Key :type Key%20Structure))
  ;[1 1 1] Hold movement
  (:Pressed
    (Variables|Default|SetCanMove? true))
  (:Released
    (Variables|Default|SetCanMove? false)))

(event Input|MouseEvents|MouseWheelUp
  (params (Key :type Key%20Structure))
  (bind _springarm (Variables|Default|GetSpringArm))
  ;[1 1 1] Zoom
  (:Pressed
    (Variables|/Script/Engine.SpringArmComponent|SetTargetArmLength _springarm (- (Variables|/Script/Engine.SpringArmComponent|GetTargetArmLength _springarm) (Variables|Default|GetZoomSpeed)))))

(event Input|MouseEvents|MouseWheelDown
  (params (Key :type Key%20Structure))
  (bind _springarm (Variables|Default|GetSpringArm))
  ;[1 1 1] Zoom
  (:Pressed
    (Variables|/Script/Engine.SpringArmComponent|SetTargetArmLength _springarm (+ (Variables|/Script/Engine.SpringArmComponent|GetTargetArmLength _springarm) (Variables|Default|GetZoomSpeed)))))